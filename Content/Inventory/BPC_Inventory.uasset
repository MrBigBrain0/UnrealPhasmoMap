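; Inventory component for the first-person character: a four-slot hotbar holding items, with one slot selected at a time.
; On BeginPlay, the locally controlled owner creates the inventory widget, which mirrors selection and slot icons.
; Mouse wheel cycles slots with wraparound and SwapSlot selects by index, both updating the character's held mesh.
; Helper functions store, query or clear the selected slot, though IsSlotFree returns false even after storing an item.
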(event EventBeginPlay
  ;[0.15 0.15 0.15 0.5] Check if teh player is local, Then show the inventory
  (if (Pawn|IsLocallyControlled (Variables|/Script/Engine.Actor|GetInstigator (Components|GetOwner)))
    (bind _asbp_first_person_character (Utilities|Casting|CastToBP_FirstPersonCharacter (Components|GetOwner)))
    (Variables|Default|SetOwnerReference _asbp_first_person_character)
    (bind _returnvalue (Game|ConstructObjectfromClass "/Game/Inventory/Widgets/WBP_InventoryWidget.WBP_InventoryWidget_C"))
    (bind _output_get (Variables|Default|SetInventoryWdget _returnvalue))
    (UserInterface|Viewport|AddtoViewport _output_get 0)
    (Default|HighlightSlot (Variables|Default|GetInventoryWdget))))

(event Input|MouseEvents|MouseWheelUp
  (params (Key :type Key%20Structure :default "None"))
  (:Pressed
    (Default|UnhighlightSlot (Variables|Default|GetInventoryWdget) (Variables|Default|GetCurrentSlotIndex))
    (bind _output_get (Variables|Default|SetCurrentSlotIndex (+ (Variables|Default|GetCurrentSlotIndex) 1)))
    (if (>= _output_get 4)
      (bind _output_get_2 (Variables|Default|SetCurrentSlotIndex 0))
      (Default|HighlightSlot (Variables|Default|GetInventoryWdget) _output_get_2)
      (else
        (Default|HighlightSlot (Variables|Default|GetInventoryWdget) (Variables|Default|GetCurrentSlotIndex))))
    (CallFunction|ChangeSlotMesh)))

(event Input|MouseEvents|MouseWheelDown
  (params (Key :type Key%20Structure :default "None"))
  (:Pressed
    (Default|UnhighlightSlot (Variables|Default|GetInventoryWdget) (Variables|Default|GetCurrentSlotIndex))
    (bind _output_get (Variables|Default|SetCurrentSlotIndex (- (Variables|Default|GetCurrentSlotIndex) 1)))
    (if (<= _output_get -1)
      (bind _output_get_2 (Variables|Default|SetCurrentSlotIndex 3))
      (Default|HighlightSlot (Variables|Default|GetInventoryWdget) _output_get_2)
      (else
        (Default|HighlightSlot (Variables|Default|GetInventoryWdget) (Variables|Default|GetCurrentSlotIndex))))
    (CallFunction|ChangeSlotMesh)))

(fn SwapSlot
  (params (SlotIndex :type Integer))
  (Default|UnhighlightSlot (Variables|Default|GetInventoryWdget) (Variables|Default|GetCurrentSlotIndex))
  (bind _output_get (Variables|Default|SetCurrentSlotIndex SlotIndex))
  (Default|HighlightSlot (Variables|Default|GetInventoryWdget) _output_get)
  (CallFunction|ChangeSlotMesh))

(fn IsSlotFree
  (params (Item :type PDA%20Items%20Object%20Reference))
  (if (== (Utilities|Array|Get(acopy) (Variables|Default|GetInventorySlots) (Variables|Default|GetCurrentSlotIndex)) 0)
    (Utilities|Array|SetArrayElem (Variables|Default|GetInventorySlots) (Variables|Default|GetCurrentSlotIndex) Item)
    (Default|SlotChanged (Variables|Default|GetInventoryWdget) (Variables|Default|GetCurrentSlotIndex) (Variables|/Game/Inventory/Pickups/Data/PDA_Items.PDA_Items_C|GetObjectImage Item) false)
    (return false)
    (else
      (return false))))

(fn QueryInventory
  (bind _inventoryslots (Variables|Default|GetInventorySlots))
  (bind _currentslotindex (Variables|Default|GetCurrentSlotIndex))
  (bind _output (Utilities|Array|Get(acopy) _inventoryslots _currentslotindex))
  (if (== _output 0)
    (return false 0)
    (else
      (return true (Variables|/Game/Inventory/Pickups/Data/PDA_Items.PDA_Items_C|GetObjectActor _output)))))

(fn RemovefromInventory
  (Utilities|Array|SetArrayElem (Variables|Default|GetInventorySlots) (Variables|Default|GetCurrentSlotIndex) 0)
  (Default|SlotChanged (Variables|Default|GetInventoryWdget) (Variables|Default|GetCurrentSlotIndex) 0 true)
  (return))

(fn ChangeSlotMesh
  (bind _inventoryslots (Variables|Default|GetInventorySlots))
  (bind _currentslotindex (Variables|Default|GetCurrentSlotIndex))
  (bind _output (Utilities|Array|Get(acopy) _inventoryslots _currentslotindex))
  (Default|ChangeHeldItem (Variables|Default|GetOwnerReference) (select (== _output 0) 0 (Variables|/Game/Inventory/Pickups/Data/PDA_Items.PDA_Items_C|GetObjectMesh _output))))